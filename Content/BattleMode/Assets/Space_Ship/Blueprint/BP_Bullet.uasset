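; BP_Bullet is the bullet actor among the battle mode space ship assets, handling impact effects and its own removal.
; On BeginPlay its Box collision is switched off, then enabled for query and physics after a very short delay.
; On a hit, it spawns a hit effect system at the impact point, oriented along the surface normal, then destroys itself after a brief delay.
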(event OnComponentHit(Box)
  (params (HitComponent :type Primitive%20Component%20Object%20Reference) (OtherActor :type Actor%20Object%20Reference) (OtherComp :type Primitive%20Component%20Object%20Reference) (NormalImpulse :type Vector :default "0, 0, 0") (Hit :type Hit%20Result%20Structure%20%28by%20ref%29))
  (bind (_bblockinghit _binitialoverlap _time _distance _location _impactpoint _normal _impactnormal) (Collision|BreakHitResult Hit))
  (Niagara|SpawnSystematLocation "/Game/BattleMode/Assets/Space_Ship/FX/NS_Hit_Effect_System.NS_Hit_Effect_System" _location (Math|Conversions|RotationFromXVector _impactnormal))
  (Utilities|FlowControl|Delay 0.2)
  (Actor|DestroyActor))

(event EventBeginPlay
  (Collision|SetCollisionEnabled (Variables|Default|GetBox) "NoCollision")
  (Utilities|FlowControl|Delay 0.02)
  (Collision|SetCollisionEnabled (Variables|Default|GetBox) "QueryAndPhysics"))

(fn ConstructionScript)