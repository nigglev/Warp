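; Procedural asteroid ring actor that spins slowly or quickly around its local Z axis on Tick, set by a rotation speed.
; The construction script fills a Hierarchical Instanced Static Mesh over a length-by-width grid, with configurable mesh and cull distances.
; AsteriodTR wraps the grid around the ring radius, using a random stream for position jitter and blending tangent-aligned with random rotation.
; Instance scale grows with width index, starting at zero.
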(event EventBeginPlay)

(event Collision|EventActorBeginOverlap
  (params (OtherActor :type Actor%20Object%20Reference)))

(event EventTick
  (params (DeltaSeconds :type Float%20%28single-precision%29))
  (Transformation|AddActorLocalRotation (Math|Vector|RotatorfromAxisandAngle "0, 0,1.000000" (* DeltaSeconds (Variables|Default|GetRotationSpeed))) false false))

(fn ConstructionScript
  (bind _hierarchicalinstancedstaticmesh (Variables|Default|GetHierarchicalInstancedStaticMesh))
  (bind _instanseconthwith (Variables|Default|GetInstanseConthWith))
  (bind _instanseconthlingeth (Variables|Default|GetInstanseConthLingeth))
  (Utilities|FlowControl|Sequence
    (:then_0
      (Components|StaticMesh|SetStaticMesh _hierarchicalinstancedstaticmesh (Variables|Default|GetMesh)))
    (:then_1
      (Components|InstancedStaticMesh|SetCullDistances _hierarchicalinstancedstaticmesh (Variables|Default|GetCollingNear) (Variables|Default|GetCollingFar)))
    (:then_2
      (for _index (range 0 (- _instanseconthlingeth 1))
        (for _index_2 (range 0 (- _instanseconthwith 1))
          (bind (_o_location _o_rotation) (CallFunction|AsteriodTR _index_2 _instanseconthwith _index _instanseconthlingeth))
          (Components|InstancedStaticMesh|AddInstance (Variables|Default|GetHierarchicalInstancedStaticMesh) (Math|Transform|MakeTransform _o_location _o_rotation (Math|Conversions|ToVector(Float) (* (Math|Conversions|ToFloat(Integer) _index_2) (Variables|Default|GetRandomScaleMinimur))))))))))

(fn AsteriodTR
  (params (Index%20Width%20Loop :type Integer) (NumberInstanseWidth :type Integer) (IndexLingethLoop :type Integer) (NumberInstanseLingeth :type Integer))
  (bind _returnvalue (Math|Conversions|ToFloat(Integer) NumberInstanseWidth))
  (bind _returnvalue_2 (Math|Vector|MakeVector 0.0 0.0 1.0))
  (bind _returnvalue_3 (Math|Conversions|ToFloat(Integer) IndexLingethLoop))
  (bind _returnvalue_4 (Math|Conversions|ToFloat(Integer) NumberInstanseLingeth))
  (bind _returnvalue_5 (Math|Float|MakeLiteralFloat 3.6e+02))
  (bind _returnvalue_6 (Math|Conversions|ToFloat(Integer) Index%20Width%20Loop))
  (bind _transforamarandome (Variables|Default|GetTransforamaRandome))
  (bind _randomaseposychane (Variables|Default|GetRandomasePosychane))
  (bind _randomzaxisposit (Variables|Default|GetRandomZAxisPosit))
  (bind _ringwith (Variables|Default|GetRingWith))
  (bind _ringwith_2 (Variables|Default|GetRingWith))
  (bind _ridois (Variables|Default|GetRidois))
  (bind _returnvalue_7 (Math|Random|RandomFloatfromStream _transforamarandome))
  (bind _returnvalue_8 (Math|Random|RandomUnitVectorfromStream _transforamarandome))
  (bind _returnvalue_9 (/ _returnvalue_3 _returnvalue_4))
  (bind _returnvalue_10 (/ _returnvalue_6 _returnvalue))
  (bind _returnvalue_11 (- _returnvalue_10 0.5))
  (bind _returnvalue_12 (- _returnvalue_7 0.5))
  (bind _returnvalue_13 (* _returnvalue_8 _randomaseposychane))
  (bind _returnvalue_14 (* _returnvalue_9 _returnvalue_5))
  (bind _returnvalue_15 (* _returnvalue_12 _randomzaxisposit _ringwith))
  (bind _returnvalue_16 (* _returnvalue_11 _ringwith_2))
  (bind _returnvalue_17 (Math|Conversions|ToVector(Float) _returnvalue_15))
  (bind _returnvalue_18 (+ _ridois _returnvalue_16))
  (bind _returnvalue_19 (Math|Vector|MakeVector 0.0 _returnvalue_18 0.0))
  (bind _returnvalue_20 (+ _returnvalue_17 _returnvalue_13))
  (bind _returnvalue_21 (+ _returnvalue_20 _returnvalue_19))
  (bind _returnvalue_22 (Math|Vector|RotateVectorAroundAxis _returnvalue_21 _returnvalue_14 _returnvalue_2))
  (return _returnvalue_22 (Math|Rotator|Lerp(Rotator) (Class|KismetMathLibrary|MakeRotfromYZ (Math|Vector|CrossProduct _returnvalue_2 _returnvalue_22) _returnvalue_2) (Class|KismetMathLibrary|RandomRotatorfromStream true (Variables|Default|GetTransforamaRandome)) (Variables|Default|GetRandomRotation) true)))